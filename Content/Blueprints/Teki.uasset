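; Teki is an AI controller that sends its controlled Enemy pawn around a looping set of patrol points.
; On BeginPlay it casts the pawn to Enemy and copies that pawn's patrol point array.
; GoToPatrol moves the pawn to the current point; on success it advances the index with modulo wraparound and calls a timer targeting itself.
; Nothing in this graph makes the first GoToPatrol call.
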(event Custom|GoToPatrol
  (AI|AIMoveTo (Pawn|GetControlledPawn) (CallFunction|GetPatrolLocation) 0 5.0 false
    (:OnSuccess
      (CallFunction|PopPatrolLocation)
      (Utilities|Time|SetTimerbyFunctionName 0 "GoToPatrol" 0.0))))

(event EventBeginPlay
  (bind _asenemy (Utilities|Casting|CastToEnemy (Pawn|GetControlledPawn)))
  (Variables|Default|SetAI_PatrolPoints (Variables|/Game/Blueprints/Enemy.Enemy_C|GetPatorlPoint _asenemy)))

(event EventTick
  (params (DeltaSeconds :type Float%20%28single-precision%29)))

(fn ConstructionScript)

(fn GetPatrolLocation
  (return (Transformation|GetActorLocation (Utilities|Array|Get(acopy) (Variables|Default|GetAI_PatrolPoints) (Variables|Default|GetPatrolIndex)))))

(fn PopPatrolLocation
  (Variables|Default|SetPatrolIndex (Math|Integer|%(Integer) (+ (Variables|Default|GetPatrolIndex) 1) (Utilities|Array|Length (Variables|Default|GetAI_PatrolPoints)))))